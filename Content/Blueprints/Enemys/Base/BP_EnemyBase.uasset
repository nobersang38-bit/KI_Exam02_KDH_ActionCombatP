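; BP_EnemyBase is a base enemy Blueprint that provides a montage-based attack interface and hides its OnTargeting indicator at BeginPlay.
; AttackPlay passes an index to AttackPlayEvent, which plays that entry of AttackMontages on the Mesh, and returns false for both IsComplete and AttackFail without waiting for the montage.
; EnableAttackIDX is a stub that always returns -1, so attack selection is not implemented here.
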(event `self.ReceiveBeginPlay`
  (`SceneComponent.SetVisibility` (`self.OnTargeting`) false false))

(event `AttackPlayEvent`
  (params (AttackIDX :type Integer))
  (`|PlayMontage` (`self.Mesh`) (`|GetArrayItem` (`self.AttackMontages`) AttackIDX)))

(fn `AttackPlay`
  (params (AttackIDX :type Integer))
  (returns (IsComplete :type Boolean) (AttackFail :type Boolean))
  (`self.AttackPlayEvent` AttackIDX)
  (return false false))

(fn `EnableAttackIDX`
  (returns (AttackIDX :type Integer))
  (return -1))

(fn `UserConstructionScript`)