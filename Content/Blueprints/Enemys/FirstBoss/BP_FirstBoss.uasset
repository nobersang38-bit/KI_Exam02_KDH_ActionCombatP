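; First boss enemy that attacks the player with random montages and is destroyed when its health runs out.
; Attackkk drives timelines that turn and move it toward the player, with a homing lunge for attack index 4.
; ONC/OffC events toggle the attack hitbox, which Tick also disables after a parry or completed attack.
; Weapon overlaps or InDamage reduce BPCombatSystem health by evade type, updating a camera-facing health bar and playing a hit montage.
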(event `self.ReceiveBeginPlay`
  (`parent.ReceiveBeginPlay`)
  (`PrimitiveComponent.SetCollisionEnabled` (`self.AttackCollision`) "NoCollision"))

(event `self.ReceiveTick`
  (params (DeltaSeconds :type "Float (single-precision)"))
  (`parent.ReceiveTick` DeltaSeconds)
  (`|ExecutionSequence`
    (:`then_0`
      (if (or (`self.IsParryHit`) (`self.IsAttackComplete`))
        (`PrimitiveComponent.SetCollisionEnabled` (`self.AttackCollision`) "NoCollision")))
    (:`then_1`
      (bind _asbp_main_player (cast `/Game/Blueprints/MainPlayer/BP_MainPlayer` (`GameplayStatics.GetPlayerCharacter` 0)))
      (`SceneComponent.K2_SetWorldRotation` (`self.Widget`) (`KismetMathLibrary.MakeRotFromX` (- (`SceneComponent.K2_GetComponentLocation` (`/Game/Blueprints/MainPlayer/BP_MainPlayer.Camera` _asbp_main_player)) (`SceneComponent.K2_GetComponentLocation` (`self.Widget`)))) false false))))

(event `Attackkk`
  (bind _returnvalue (`self.K2_GetActorLocation`))
  (bind _returnvalue_2 (`GameplayStatics.GetWorldDeltaSeconds`))
  (bind (_returnvalue_roll _returnvalue_pitch _returnvalue_yaw) (`KismetMathLibrary.BreakRotator` (`self.K2_GetActorRotation`)))
  (bind _returnvalue_3 (`GameplayStatics.GetPlayerPawn` 0))
  (bind (_returnvalue_x _returnvalue_y) (`KismetMathLibrary.BreakVector` (`self.K2_GetActorLocation`)))
  (bind _attackmontages (`self.AttackMontages`))
  (bind _returnvalue_4 (`self.K2_GetActorLocation` (`GameplayStatics.GetPlayerPawn` 0)))
  (bind (_returnvalue_x_2 _returnvalue_y_2) (`KismetMathLibrary.BreakVector` (`self.K2_GetActorLocation` _returnvalue_3)))
  (bind _returnvalue_5 (- (`KismetMathLibrary.MakeVector` _returnvalue_x_2 _returnvalue_y_2) (`KismetMathLibrary.MakeVector` _returnvalue_x _returnvalue_y)))
  (bind (_returnvalue_roll_2 _returnvalue_pitch_2 _returnvalue_yaw_2) (`KismetMathLibrary.BreakRotator` (`KismetMathLibrary.MakeRotFromX` (- _returnvalue_4 _returnvalue))))
  (bind (_returnvalue_roll_3 _returnvalue_pitch_3 _returnvalue_yaw_3) (`KismetMathLibrary.BreakRotator` (`KismetMathLibrary.RInterpTo` (`KismetMathLibrary.MakeRotator` 0.0 0.0 _returnvalue_yaw) (`KismetMathLibrary.MakeRotator` 0.0 0.0 _returnvalue_yaw_2) _returnvalue_2 50.0)))
  (bind _output_get (set `self.RandomInt` (`KismetMathLibrary.RandomIntegerInRange` 0 (- (`KismetArrayLibrary.Array_Length` _attackmontages) 1))))
  (`|PlayMontage` (`self.Mesh`) (`|GetArrayItem` _attackmontages _output_get) 0.5 0.0 "None" false
    (:`then`
      (`|ExecutionSequence`
        (:`then_0`
          (`KismetSystemLibrary.PrintString` (`KismetStringLibrary.Conv_IntToString` _output_get))
          (`Timeline|타임라인` :!via `PlayFromStart`
            (:`Update`
              (`/Engine/EditorBlueprintResources/StandardMacros.IsValid` _returnvalue_3
                (:`Is Valid`
                  (`self.K2_SetActorRotation` (`KismetMathLibrary.RInterpTo` (`self.K2_GetActorRotation`) (`KismetMathLibrary.MakeRotFromX` _returnvalue_5) (`GameplayStatics.GetWorldDeltaSeconds`) 7.5))
                  (`PawnMovementComponent.AddInputVector` (`self.CharacterMovement`) _returnvalue_5 false))))))
        (:`then_1`
          (switch `int` _output_get
            (:`4`
              (bind (_direction `_새_트랙_0`) (`Timeline|타임라인_0` :!via `PlayFromStart`)
                (:`Update`
                  (if (> `_새_트랙_0` 0.5)
                    (`self.K2_SetActorLocation` (`KismetMathLibrary.VInterpTo` _returnvalue _returnvalue_4 _returnvalue_2 (* `_새_트랙_0` 1000.0)) true))
                  (`self.K2_SetActorRotation` (`KismetMathLibrary.MakeRotator` 0.0 0.0 _returnvalue_yaw_3)))))))))
    (:`OnCompleted`
      (set `self.IsAttackComplete` true))))

(event `ONC`
  (`PrimitiveComponent.SetCollisionEnabled` (`self.AttackCollision`) "QueryAndPhysics"))

(event `OffC`
  (`PrimitiveComponent.SetCollisionEnabled` (`self.AttackCollision`) "NoCollision"))

(event `self.CapsuleComponent.OnComponentBeginOverlap`
  (params (OverlappedComponent :type "PrimitiveComponent Object Reference") (OtherActor :type "Actor Object Reference") (OtherComp :type "PrimitiveComponent Object Reference") (OtherBodyIndex :type Integer) (bFromSweep :type Boolean) (SweepResult :type "HitResult Structure (by ref)"))
  (bind _bp_combatsystem (`self.BP_CombatSystem`))
  (if (`ActorComponent.ComponentHasTag` OtherComp "Weapon")
    (switch `/Game/Blueprints/Combat/E_EvadeType` (`/Game/Blueprints/Combat/BP_CombatSystem_Component.CurrentEvadeType` _bp_combatsystem) :!label _label
      (:`NewEnumerator6`
        (set `/Game/Blueprints/Combat/BP_CombatSystem_Component.CurrentHealth` (- (`/Game/Blueprints/Combat/BP_CombatSystem_Component.CurrentHealth` _bp_combatsystem) 10.0) _bp_combatsystem))
      (:`NewEnumerator3`
        (set `/Game/Blueprints/Combat/BP_CombatSystem_Component.CurrentHealth` (- (`/Game/Blueprints/Combat/BP_CombatSystem_Component.CurrentHealth` _bp_combatsystem) 5.0) _bp_combatsystem)))
    (bind _aswb_health_bar (cast `/Game/Widget/WB_HealthBar` (`WidgetComponent.GetWidget` (`self.Widget`))))
    (`/Game/Widget/WB_HealthBar.SetPercent` _aswb_health_bar (/ (`/Game/Blueprints/Combat/BP_CombatSystem_Component.CurrentHealth` _bp_combatsystem) (`/Game/Blueprints/Combat/BP_CombatSystem_Component.MaxHealth` _bp_combatsystem)))
    (`|PlayMontage` (`self.Mesh`) "/Game/Characters/Urban_Nomad/Animation/Hit/ARPG_Samurai_Anim_Samurai_Hit3_Montage.ARPG_Samurai_Anim_Samurai_Hit3_Montage" 1.0 0.0 "None" false
      (:`then`
        (if (<= (`/Game/Blueprints/Combat/BP_CombatSystem_Component.CurrentHealth` _bp_combatsystem) 0.0)
          (`self.K2_DestroyActor`))))))

(event `InDamage`
  (goto _label))

(event `AttackFalse`
  (set `self.IsAttackComplete` true))

(fn `AttackPlay`
  (params (AttackIDX :type Integer))
  (returns (IsComplete :type Boolean) (AttackFail :type Boolean))
  (switch `int` AttackIDX))

(fn `EnableAttackIDX`
  (returns (AttackIDX :type Integer))
  (return -1))

(fn `UserConstructionScript`
  (`parent.UserConstructionScript`))