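; Combat component that tracks health, stamina and evade state, and resolves incoming damage for its owner.
; Damage avoids health loss when the current evade type is among the hit's evadable types, unless it is flagged CantEvade.
; Otherwise it reduces health and drains stamina by groggy damage.
; Dispatchers report the evade type, death or attack strength, while SendDamage helpers forward damage info to target actors by message.
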(event `self.ReceiveBeginPlay`
  (set `self.CurrentHealth` (`self.MaxHealth`)))

(event `self.ReceiveTick`
  (params (DeltaSeconds :type "Float (single-precision)")))

(event `/Game/Blueprints/Combat/BPI_InDamage.InDamage`
  (params (InDamageInfo :type "/Game/Blueprints/Combat/ST_DamageInfo Structure"))
  (`self.Internal_InDamage` InDamageInfo))

(fn `Debug_InDamage`
  (params (InDamage :type "/Game/Blueprints/Combat/ST_DamageInfo Structure"))
  (`self.Internal_InDamage` InDamage))

(fn `GetCurrentEvade`
  (returns (EvadeType :type "/Game/Blueprints/Combat/E_EvadeType Enum"))
  (return (`self.CurrentEvadeType`)))

(fn `Internal_InDamage`
  (params (DamageInfo :type "/Game/Blueprints/Combat/ST_DamageInfo Structure"))
  (locals (IsSuccessEvade :type Boolean))
  (if (`KismetMathLibrary.BooleanNOR` (`BlueprintSetLibrary.Set_Contains` DamageInfo_EvadeType_26_22EBE451468C10F538B3499F20FB03E0 "NewEnumerator1") (== (`KismetMathLibrary.Conv_ByteToInt` (`self.CurrentEvadeType`)) (`KismetMathLibrary.Conv_ByteToInt` (enumliteral `/Game/Blueprints/Combat/E_EvadeType` "NewEnumerator6"))))
    (bind _result (`BlueprintSetLibrary.Set_ToArray` DamageInfo_EvadeType_26_22EBE451468C10F538B3499F20FB03E0))
    (for _array_element _result
      (if (== (`KismetMathLibrary.Conv_ByteToInt` _array_element) (`KismetMathLibrary.Conv_ByteToInt` (`self.CurrentEvadeType`)))
        (set `local.IsSuccessEvade` true)
        (break)))
    (if (`local.IsSuccessEvade`)
      (switch `/Game/Blueprints/Combat/E_EvadeType` (`self.CurrentEvadeType`)
        (:`NewEnumerator6`
          (`self.InDamage_EvadeType_None`))
        (:`NewEnumerator1`
          (`self.InDamage_EvadeType_CantEvade`))
        (:`NewEnumerator2`
          (`self.InDamage_EvadeType_Evasion`))
        (:`NewEnumerator3`
          (`self.InDamage_EvadeType_Deffense`))
        (:`NewEnumerator4`
          (`self.InDamage_EvadeType_PerfectGaurd`))
        (:`NewEnumerator5`
          (`self.InDamage_EvadeType_Gimmick`)))
      (else
        (bind _output_get (set `self.CurrentHealth` (`KismetMathLibrary.FClamp` (- (`self.CurrentHealth`) DamageInfo_Health_Damage_2_92C3AE2A462AE5A7DFB148B2F3494F72) 0.0 1000000000.0) :!label _label))
        (set `self.Stamina` (`KismetMathLibrary.FClamp` (- (`self.Stamina`) DamageInfo_Groggy_Damage_4_60E9581640CA749D1EDDB59C7F15D5BC) 0.0 1000000000.0))
        (if (<= _output_get 0.0)
          (`self.InDamage_Death`)
          (else
            (switch `/Game/Blueprints/Combat/E_DamageType` DamageInfo_DamageType_7_8F5477C3412F404F6E01D4BF37E8D7C2
              (:`NewEnumerator0`
                (`self.InDamage_DamageType_None`))
              (:`NewEnumerator1`
                (`self.InDamage_DamageType_WeakAttack`))
              (:`NewEnumerator2`
                (`self.InDamage_DamageType_NormalAttack`))
              (:`NewEnumerator3`
                (`self.InDamage_DamageType__PowerAttack`))
              (:`NewEnumerator4`
                (`self.InDamage_DamageType_SuperPowerAttack`)))))))
    (else
      (goto _label))))

(fn `SendDamage_FindActor`
  (params (DamageInfo :type "/Game/Blueprints/Combat/ST_DamageInfo Structure") (TargetActor :type "Actor Object Reference") (NewParam :type "Actor Object Reference"))
  (message `/Game/Blueprints/Combat/BPI_InDamage.InDamage` TargetActor DamageInfo))

(fn `SendDamage_FindIDX`
  (params (DamageInfo :type "/Game/Blueprints/Combat/ST_DamageInfo Structure") (TargetActor :type "Actor Object Reference"))
  (message `/Game/Blueprints/Combat/BPI_InDamage.InDamage` TargetActor DamageInfo))

(fn `SendDamage_FindString`
  (params (DamageInfo :type "/Game/Blueprints/Combat/ST_DamageInfo Structure") (TargetActor :type "Actor Object Reference"))
  (message `/Game/Blueprints/Combat/BPI_InDamage.InDamage` TargetActor DamageInfo))

(fn `SetCurrentEvade`
  (params (EvadeType :type "/Game/Blueprints/Combat/E_EvadeType Enum" :default "NewEnumerator0"))
  (set `self.CurrentEvadeType` EvadeType))