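; Player controller for the main player that sets up Enhanced Input and handles quitting the game.
; BeginPlay adds the mapping context at priority 0, and completing IA_GameExit quits.
; An unconnected chain would rebuild FindMoveChecker mappings by removing existing entries in reverse index order, then re-adding copies of FindMove's keys, triggers and modifiers; it never runs.
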(event `self.ReceiveBeginPlay`
  (`EnhancedInputSubsystemInterface.AddMappingContext` (subsystem `EnhancedInputLocalPlayerSubsystem`) (`self.Mapping Context`) 0 (struct)))

(event `EnhancedInput|/Game/Input/IA_GameExit`
  (params (ActionValue :type Boolean) (ElapsedSeconds :type "Float (double-precision)") (TriggeredSeconds :type "Float (double-precision)") (InputAction :type "InputAction Object Reference" :default "/Game/Input/IA_GameExit.IA_GameExit"))
  (:`Completed`
    (`KismetSystemLibrary.QuitGame` null "Quit")))

(fn `UserConstructionScript`)