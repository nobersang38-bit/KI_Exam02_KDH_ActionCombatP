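; Main player component that decides when a new motion may start from the current one, including combo steps.
; MotionsInfo maps each motion to combo data and timing windows for allowed next motions.
; MotionStartCheck tests elapsed time against a window or default time, advances or resets the combo index, and returns success and index.
; Tick runs the timer and expires combos to -1; MotionALLReset rebuilds the map with zeroed timings.
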(event `self.ReceiveBeginPlay`
  (set `self.MainPlayerMotion_FirstIDX` (+ (`KismetMathLibrary.Conv_ByteToInt` (`self.MainPlayerMotion_FirstIDX_Enum`)) 0))
  (set `self.MainPlayerMotion_LastIDX` (- (`KismetMathLibrary.Conv_ByteToInt` (`self.MainPlayerMotion_LastIDX_Enum`)) 1)))

(event `self.ReceiveTick`
  (params (DeltaSeconds :type "Float (single-precision)"))
  (bind _currentmotion (`self.CurrentMotion`))
  (bind (_value _returnvalue) (`BlueprintMapLibrary.Map_Find` (`self.MotionsInfo`) _currentmotion))
  (set `self.CurrentTime` (+ DeltaSeconds (`self.CurrentTime`)))
  (if _returnvalue
    (bind _iscombo (`self.ComboMotionCheck` (break `/Game/Blueprints/MainPlayer/ST_MainPlayer_ComboInfo` (break `/Game/Blueprints/MainPlayer/ST_Motion_Struct_Parent` _value))))
    (if (and _iscombo (>= (`self.CurrentTime`) (`.DefaultTime_25_1B7D5B224D372822620BE098464AABD7` (break `/Game/Blueprints/MainPlayer/ST_Motion_Struct_Child` (`BlueprintMapLibrary.Map_Find` (`.Next_MotionsEnableCheck_30_6F7DE66442D9384DFC21BFA6EA74B8C9` (break `/Game/Blueprints/MainPlayer/ST_Motion_Struct_Parent` _value)) _currentmotion)))))
      (`BlueprintMapLibrary.Map_Add` (`self.MotionsInfo`) (`self.CurrentMotion`) (make `/Game/Blueprints/MainPlayer/ST_Motion_Struct_Parent` (make `/Game/Blueprints/MainPlayer/ST_MainPlayer_ComboInfo` (break `/Game/Blueprints/MainPlayer/ST_MainPlayer_ComboInfo` (break `/Game/Blueprints/MainPlayer/ST_Motion_Struct_Parent` _value)) (`.ComboCount_6_D4D4C53D441D689F58B207A76EF3BC75` (break `/Game/Blueprints/MainPlayer/ST_MainPlayer_ComboInfo` (break `/Game/Blueprints/MainPlayer/ST_Motion_Struct_Parent` _value))) -1 (`.ComboSet_14_C02CBBA148F408893CD640AAC5C189D4` (break `/Game/Blueprints/MainPlayer/ST_MainPlayer_ComboInfo` (break `/Game/Blueprints/MainPlayer/ST_Motion_Struct_Parent` _value)))) (`.Next_MotionsEnableCheck_30_6F7DE66442D9384DFC21BFA6EA74B8C9` (break `/Game/Blueprints/MainPlayer/ST_Motion_Struct_Parent` _value)))))))

(fn `ComboMotionCheck`
  (params (ComboType :type "/Game/Blueprints/MainPlayer/E_MainPlayer_ComboType Enum" :default "NewEnumerator0"))
  (returns (IsCombo :type Boolean))
  (if (and (!= (`KismetMathLibrary.Conv_ByteToInt` (enumliteral `/Game/Blueprints/MainPlayer/E_MainPlayer_ComboType` "NewEnumerator1")) (`KismetMathLibrary.Conv_ByteToInt` ComboType)) (!= (`KismetMathLibrary.Conv_ByteToInt` (enumliteral `/Game/Blueprints/MainPlayer/E_MainPlayer_ComboType` "NewEnumerator0")) (`KismetMathLibrary.Conv_ByteToInt` ComboType)))
    (return true)
    (else
      (return false))))

(fn `MotionALLReset`
  (locals (Temp :type "Array of /Game/Blueprints/MainPlayer/ST_Motion_Struct_Child Structure"))
  (for _index (range (`self.MainPlayerMotion_FirstIDX`) (+ (`self.MainPlayerMotion_LastIDX`) 1))
    (`BlueprintMapLibrary.Map_Add` (`self.TempChilds`) (cast `/Game/Blueprints/MainPlayer/E_MainPlayer_Motion` (`KismetMathLibrary.Conv_IntToByte` _index)) (make `/Game/Blueprints/MainPlayer/ST_Motion_Struct_Child` (0.0 0.0))))
  (for _index_2 (range (`self.MainPlayerMotion_FirstIDX`) (+ (`self.MainPlayerMotion_LastIDX`) 1))
    (bind _returnvalue (cast `/Game/Blueprints/MainPlayer/E_MainPlayer_Motion` (`KismetMathLibrary.Conv_IntToByte` _index_2)))
    (bind _value (`BlueprintMapLibrary.Map_Find` (`self.MotionsInfo`) _returnvalue))
    (bind _iscombo (`self.ComboMotionCheck` (break `/Game/Blueprints/MainPlayer/ST_MainPlayer_ComboInfo` (break `/Game/Blueprints/MainPlayer/ST_Motion_Struct_Parent` _value))))
    (if _iscombo
      (`KismetArrayLibrary.Array_Clear` (`local.Temp`))
      (for _ (range (`.ComboCount_6_D4D4C53D441D689F58B207A76EF3BC75` (break `/Game/Blueprints/MainPlayer/ST_MainPlayer_ComboInfo` (break `/Game/Blueprints/MainPlayer/ST_Motion_Struct_Parent` _value))))
        (`KismetArrayLibrary.Array_Add` (`local.Temp`) (make `/Game/Blueprints/MainPlayer/ST_Motion_Struct_Child` (0.0 0.0))))
      (`BlueprintMapLibrary.Map_Add` (`self.MotionsInfo`) _returnvalue (make `/Game/Blueprints/MainPlayer/ST_Motion_Struct_Parent` (make `/Game/Blueprints/MainPlayer/ST_MainPlayer_ComboInfo` (break `/Game/Blueprints/MainPlayer/ST_MainPlayer_ComboInfo` (break `/Game/Blueprints/MainPlayer/ST_Motion_Struct_Parent` _value)) (`.ComboCount_6_D4D4C53D441D689F58B207A76EF3BC75` (break `/Game/Blueprints/MainPlayer/ST_MainPlayer_ComboInfo` (break `/Game/Blueprints/MainPlayer/ST_Motion_Struct_Parent` _value))) 0 (`local.Temp`)) (`self.TempChilds`)))
      (else
        (`BlueprintMapLibrary.Map_Add` (`self.MotionsInfo`) _returnvalue (make `/Game/Blueprints/MainPlayer/ST_Motion_Struct_Parent` (make `/Game/Blueprints/MainPlayer/ST_MainPlayer_ComboInfo` (break `/Game/Blueprints/MainPlayer/ST_MainPlayer_ComboInfo` (break `/Game/Blueprints/MainPlayer/ST_Motion_Struct_Parent` _value)) -1 -1 _) (`self.TempChilds`)))))))

(fn `MotionStartCheck`
  (params (ThisMotion :type "/Game/Blueprints/MainPlayer/E_MainPlayer_Motion Enum" :default "NewEnumerator5"))
  (returns (IsSuccess :type Boolean) (ComboIDX :type Integer))
  (bind (_value _returnvalue) (`BlueprintMapLibrary.Map_Find` (`self.MotionsInfo`) (`self.CurrentMotion`)))
  (bind _value_2 (`BlueprintMapLibrary.Map_Find` (`self.MotionsInfo`) (`self.CurrentMotion`)))
  (bind _value_3 (`BlueprintMapLibrary.Map_Find` (`self.MotionsInfo`) (`self.CurrentMotion`)))
  (bind _value_4 (`BlueprintMapLibrary.Map_Find` (`self.MotionsInfo`) (`self.CurrentMotion`)))
  (bind (_value_5 _returnvalue_2) (`BlueprintMapLibrary.Map_Find` (`.Next_MotionsEnableCheck_30_6F7DE66442D9384DFC21BFA6EA74B8C9` (break `/Game/Blueprints/MainPlayer/ST_Motion_Struct_Parent` _value)) ThisMotion))
  (bind _output (`|GetArrayItem` (`.ComboSet_14_C02CBBA148F408893CD640AAC5C189D4` (break `/Game/Blueprints/MainPlayer/ST_MainPlayer_ComboInfo` (break `/Game/Blueprints/MainPlayer/ST_Motion_Struct_Parent` _value_3))) (`.CurrentComboIDX_9_0DA80BF647BD08C632B0339884736E80` (break `/Game/Blueprints/MainPlayer/ST_MainPlayer_ComboInfo` (break `/Game/Blueprints/MainPlayer/ST_Motion_Struct_Parent` _value_3)))))
  (bind _returnvalue_3 (+ (`.CurrentComboIDX_9_0DA80BF647BD08C632B0339884736E80` (break `/Game/Blueprints/MainPlayer/ST_MainPlayer_ComboInfo` (break `/Game/Blueprints/MainPlayer/ST_Motion_Struct_Parent` _value))) 1))
  (if _returnvalue
    (if _returnvalue_2
      (bind _iscombo (`self.ComboMotionCheck` (break `/Game/Blueprints/MainPlayer/ST_MainPlayer_ComboInfo` (break `/Game/Blueprints/MainPlayer/ST_Motion_Struct_Parent` _value))))
      ; 콤보로 설정되어 있는건지 확인하는 겁니다
      (if _iscombo
        (if (or (!= (`KismetMathLibrary.Conv_ByteToInt` ThisMotion) (`KismetMathLibrary.Conv_ByteToInt` (`self.CurrentMotion`))) (== (`.ComboCount_6_D4D4C53D441D689F58B207A76EF3BC75` (break `/Game/Blueprints/MainPlayer/ST_MainPlayer_ComboInfo` (break `/Game/Blueprints/MainPlayer/ST_Motion_Struct_Parent` _value))) _returnvalue_3))
          (`BlueprintMapLibrary.Map_Add` (`self.MotionsInfo`) (`self.CurrentMotion`) (make `/Game/Blueprints/MainPlayer/ST_Motion_Struct_Parent` (make `/Game/Blueprints/MainPlayer/ST_MainPlayer_ComboInfo` (break `/Game/Blueprints/MainPlayer/ST_MainPlayer_ComboInfo` (break `/Game/Blueprints/MainPlayer/ST_Motion_Struct_Parent` _value_2)) (`.ComboCount_6_D4D4C53D441D689F58B207A76EF3BC75` (break `/Game/Blueprints/MainPlayer/ST_MainPlayer_ComboInfo` (break `/Game/Blueprints/MainPlayer/ST_Motion_Struct_Parent` _value_2))) 0 (`.ComboSet_14_C02CBBA148F408893CD640AAC5C189D4` (break `/Game/Blueprints/MainPlayer/ST_MainPlayer_ComboInfo` (break `/Game/Blueprints/MainPlayer/ST_Motion_Struct_Parent` _value_2)))) (`.Next_MotionsEnableCheck_30_6F7DE66442D9384DFC21BFA6EA74B8C9` (break `/Game/Blueprints/MainPlayer/ST_Motion_Struct_Parent` _value_2))))
          (else
            (`BlueprintMapLibrary.Map_Add` (`self.MotionsInfo`) (`self.CurrentMotion`) (make `/Game/Blueprints/MainPlayer/ST_Motion_Struct_Parent` (make `/Game/Blueprints/MainPlayer/ST_MainPlayer_ComboInfo` (break `/Game/Blueprints/MainPlayer/ST_MainPlayer_ComboInfo` (break `/Game/Blueprints/MainPlayer/ST_Motion_Struct_Parent` _value_4)) (`.ComboCount_6_D4D4C53D441D689F58B207A76EF3BC75` (break `/Game/Blueprints/MainPlayer/ST_MainPlayer_ComboInfo` (break `/Game/Blueprints/MainPlayer/ST_Motion_Struct_Parent` _value_4))) _returnvalue_3 (`.ComboSet_14_C02CBBA148F408893CD640AAC5C189D4` (break `/Game/Blueprints/MainPlayer/ST_MainPlayer_ComboInfo` (break `/Game/Blueprints/MainPlayer/ST_Motion_Struct_Parent` _value_4)))) (`.Next_MotionsEnableCheck_30_6F7DE66442D9384DFC21BFA6EA74B8C9` (break `/Game/Blueprints/MainPlayer/ST_Motion_Struct_Parent` _value_4))))))
        ; 콤보면 따로 계산
        (set `self.CurrentTime` 0.0)
        (set `self.CurrentMotion` ThisMotion)
        (bind _issuccess (`self.TimeCheck` (`KismetMathLibrary.BreakVector2D` (break `/Game/Blueprints/MainPlayer/ST_Motion_Struct_Child` _output)) (`.Y` (`KismetMathLibrary.BreakVector2D` (break `/Game/Blueprints/MainPlayer/ST_Motion_Struct_Child` _output))) (`.DefaultTime_25_1B7D5B224D372822620BE098464AABD7` (break `/Game/Blueprints/MainPlayer/ST_Motion_Struct_Child` _output))))
        (if _issuccess
          (return true (`.CurrentComboIDX_9_0DA80BF647BD08C632B0339884736E80` (break `/Game/Blueprints/MainPlayer/ST_MainPlayer_ComboInfo` (break `/Game/Blueprints/MainPlayer/ST_Motion_Struct_Parent` _value_3))))
          (else
            (return false 0)))
        (else
          (bind _issuccess_2 (`self.TimeCheck` (`KismetMathLibrary.BreakVector2D` (break `/Game/Blueprints/MainPlayer/ST_Motion_Struct_Child` _value_5)) (`.Y` (`KismetMathLibrary.BreakVector2D` (break `/Game/Blueprints/MainPlayer/ST_Motion_Struct_Child` _value_5))) (`.DefaultTime_25_1B7D5B224D372822620BE098464AABD7` (break `/Game/Blueprints/MainPlayer/ST_Motion_Struct_Child` _value_5))))
          (if _issuccess_2
            (set `self.CurrentTime` 0.0)
            (set `self.CurrentMotion` ThisMotion)
            ; 일반 모션들
            (return true 0)
            (else
              _))))
      (else
        (`KismetSystemLibrary.PrintString` "어라 모션정보에 이게 없나봐요" true true (struct :`R` 1.0 :`A` 1.0) :!label _label)))
    (else
      (goto _label)))
  (return false 0))

(fn `TimeCheck`
  (params (EnableTImeMin :type "Float (double-precision)") (EnableTimeMax :type "Float (double-precision)") (DefaultTIme :type "Float (double-precision)"))
  (returns (IsSuccess :type Boolean))
  (bind _currenttime (`self.CurrentTime`))
  (if (or (and (<= EnableTImeMin _currenttime) (<= _currenttime EnableTimeMax)) (<= DefaultTIme (`self.CurrentTime`)))
    (return true)
    (else
      (return false))))