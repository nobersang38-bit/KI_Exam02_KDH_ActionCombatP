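; Third-person player character with walk, sprint, jump, smoothed follow camera and enemy lock-on.
; The spring arm detaches at BeginPlay, then Tick lags it after the actor and eases its yaw toward the character's facing during sideways movement.
; Lock-on uses sphere overlap, line of sight and camera angle to pick an enemy, steering camera and non-sprinting body toward it.
; Decaying horizontal look input switches targets left or right; excess distance releases lock.
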(event `self.ReceiveBeginPlay`
  (bind _springarm (`self.SpringArm`))
  (set `CharacterMovementComponent.MaxWalkSpeed` (`self.BaseWalkSpeed`) (`self.CharacterMovement`))
  (`SceneComponent.SetVisibility` (`self.OnTargeting`) false false)
  (`SceneComponent.K2_DetachFromComponent` _springarm "KeepWorld" "KeepWorld" "KeepWorld" true)
  (set `self.FirstSpringArmLocation` (- (`SceneComponent.K2_GetComponentLocation` _springarm) (`self.K2_GetActorLocation`))))

(event `self.ReceiveTick`
  (params (DeltaSeconds :type "Float (single-precision)"))
  (bind (_returnvalue_x _returnvalue_y) (`KismetMathLibrary.BreakVector` (`self.GetVelocity`)))
  (bind _springarm (`self.SpringArm`))
  (bind _mesh (`self.Mesh`))
  (bind (_returnvalue_location _returnvalue_rotation _returnvalue_scale) (`KismetMathLibrary.BreakTransform` (`SceneComponent.K2_GetComponentToWorld` _mesh)))
  (bind (_returnvalue_roll _returnvalue_pitch _returnvalue_yaw) (`KismetMathLibrary.BreakRotator` (`SceneComponent.K2_GetComponentRotation` (`self.SpringArm`))))
  (bind (_relativerotation_roll _relativerotation_pitch _relativerotation_yaw) (`KismetMathLibrary.BreakRotator` (`SceneComponent.RelativeRotation` (`self.SpringArm`))))
  (bind (_returnvalue_roll_2 _returnvalue_pitch_2 _returnvalue_yaw_2) (`KismetMathLibrary.BreakRotator` (`KismetMathLibrary.MakeRotFromX` (`SceneComponent.GetRightVector` (`self.Mesh`)))))
  (bind (_returnvalue_roll_3 _returnvalue_pitch_3 _returnvalue_yaw_3) (`KismetMathLibrary.BreakRotator` (`KismetMathLibrary.RInterpTo` (`self.K2_GetActorRotation`) (`KismetMathLibrary.MakeRotFromX` (- (`self.K2_GetActorLocation` (`self.LookOnTargetEnemyBase`)) (`self.K2_GetActorLocation`))) (`GameplayStatics.GetWorldDeltaSeconds`) 5.0)))
  (set `self.WalkVelocity` (`KismetMathLibrary.VSize2D` (`KismetMathLibrary.MakeVector2D` _returnvalue_x _returnvalue_y)))
  (set `self.bIsFalling` (`NavMovementComponent.IsFalling` (`self.CharacterMovement`)))
  (`|ExecutionSequence`
    (:`then_0`
      ; LookOnTarget
      (if (`self.bIsLookOnTarget`)
        (`|ExecutionSequence`
          (:`then_0`
            (`/Engine/EditorBlueprintResources/StandardMacros.DoOnce` false :!label _label))
          (:`then_1`
            (`/Engine/EditorBlueprintResources/StandardMacros.IsValid` (`self.LookOnTargetEnemyBase`)
              (:`Is Valid`
                (`|ExecutionSequence`
                  (:`then_0`
                    (if (`self.bIsSprint`)
                      (set `CharacterMovementComponent.bOrientRotationToMovement` true (`self.CharacterMovement`))
                      (else
                        (set `CharacterMovementComponent.bOrientRotationToMovement` false (`self.CharacterMovement`))
                        (`self.K2_SetActorRotation` (`KismetMathLibrary.MakeRotator` 0.0 0.0 _returnvalue_yaw_3)))))
                  (:`then_1`
                    (`SceneComponent.K2_SetWorldRotation` (`self.SpringArm`) (`KismetMathLibrary.RInterpTo` (`SceneComponent.K2_GetComponentRotation` (`self.SpringArm`)) (`KismetMathLibrary.MakeRotFromX` (`KismetMathLibrary.Normal` (- (`self.K2_GetActorLocation` (`self.LookOnTargetEnemyBase`)) (`SceneComponent.K2_GetComponentLocation` (`self.SpringArm`))))) (`GameplayStatics.GetWorldDeltaSeconds`) (`self.LookOnTargetFollowSpeed`)) false false)
                    (`SceneComponent.K2_SetRelativeRotation` (`self.SpringArm`) (`KismetMathLibrary.RInterpTo` (`SceneComponent.RelativeRotation` (`self.SpringArm`)) (`KismetMathLibrary.MakeRotator` _relativerotation_roll (+ _relativerotation_pitch (* (`self.OnTargetAddRotation`) -1.0)) _relativerotation_yaw) (`GameplayStatics.GetWorldDeltaSeconds`) (`self.LookOnTargetFollowSpeed`)) false false)
                    (`SceneComponent.SetVisibility` (`/Game/Blueprints/Enemys/BP_EnemyBase.OnTargeting` (`self.LookOnTargetEnemyBase`)) true false)
                    (`|ExecutionSequence`
                      (:`then_0`
                        (set `self.OnTargetChangeEnemCurrentCursorDistance` (`KismetMathLibrary.FInterpTo_Constant` (`self.OnTargetChangeEnemCurrentCursorDistance`) 0.0 (`GameplayStatics.GetWorldDeltaSeconds`) (* (`self.OnTargetSideChangeDistance`) (`self.OnTargetSideChange_ResetSpeed`)))))
                      (:`then_1`
                        (if (> (`KismetMathLibrary.VSize` (- (`self.K2_GetActorLocation` (`self.LookOnTargetEnemyBase`)) (`self.K2_GetActorLocation`))) (`self.OnTargetDisableDistance`))
                          (set `self.bIsLookOnTarget` false)))
                      (:`then_2`
                        ;; Right
                        (if (> (`self.OnTargetChangeEnemCurrentCursorDistance`) (`self.OnTargetSideChangeDistance`))
                          (`self.LockOnEnemy_RIghtOrLeft` true)))
                      (:`then_3`
                        ;; Left
                        (if (< (`self.OnTargetChangeEnemCurrentCursorDistance`) (* (`self.OnTargetSideChangeDistance`) -1.0))
                          (`self.LockOnEnemy_RIghtOrLeft` false))))))))))
        (else
          (set `CharacterMovementComponent.bOrientRotationToMovement` true (`self.CharacterMovement`))
          (`/Engine/EditorBlueprintResources/StandardMacros.IsValid` (`self.LookOnTargetEnemyBase`)
            (:`Is Valid`
              (`SceneComponent.SetVisibility` (`/Game/Blueprints/Enemys/BP_EnemyBase.OnTargeting` (`self.LookOnTargetEnemyBase`)) false false)
              (set `self.LookOnTargetEnemyBase` null)
              (goto _label :!via `Reset`))))))
    (:`then_1`
      ; CameraRotation2BaseRotation
      (if (`self.bIsCameraMove`)
        (set `self.PlayerMoveCameraRotation2BaseRotation_SpeedIn` (`KismetMathLibrary.FInterpTo` (`self.PlayerMoveCameraRotation2BaseRotation_SpeedIn`) (`self.PlayerMoveCameraRotation2BaseRotation_Speed`) (`GameplayStatics.GetWorldDeltaSeconds`) 1.0))
        (`SceneComponent.K2_SetWorldRotation` (`self.SpringArm`) (`KismetMathLibrary.RInterpTo` (`KismetMathLibrary.MakeRotator` _returnvalue_roll _returnvalue_pitch _returnvalue_yaw) (`KismetMathLibrary.MakeRotator` _returnvalue_roll _returnvalue_pitch _returnvalue_yaw_2) (`GameplayStatics.GetWorldDeltaSeconds`) (`self.PlayerMoveCameraRotation2BaseRotation_SpeedIn`)) false false)
        (else
          (set `self.PlayerMoveCameraRotation2BaseRotation_SpeedIn` 0.0))))
    (:`then_2`
      ; CameraBaseMove
      (`SceneComponent.K2_SetWorldLocation` _springarm (`KismetMathLibrary.VInterpTo` (`SceneComponent.K2_GetComponentLocation` _springarm) (+ (`self.K2_GetActorLocation`) (`self.FirstSpringArmLocation`)) (`GameplayStatics.GetWorldDeltaSeconds`) (`self.CameraLocationFollowSpeed`)) false false))
    (:`then_3`
      ; 캐릭터 기준 벨로시티
      (`/Engine/EditorBlueprintResources/StandardMacros.IsValid` (`self.LookOnTargetEnemyBase`)
        (:`Is Valid`
          (set `self.CameraKiJunMoveVelocity` (`KismetMathLibrary.InverseTransformLocation` (`KismetMathLibrary.MakeTransform` _returnvalue_location (`KismetMathLibrary.MakeRotFromX` (`SceneComponent.GetRightVector` _mesh)) _returnvalue_scale) (+ (`SceneComponent.K2_GetComponentLocation` _mesh) (`self.GetVelocity`)))))))))

(event `EnhancedInput|/Game/Input/IA_OnTarget`
  (params (ActionValue :type Boolean) (ElapsedSeconds :type "Float (double-precision)") (TriggeredSeconds :type "Float (double-precision)") (InputAction :type "InputAction Object Reference" :default "/Game/Input/IA_OnTarget.IA_OnTarget"))
  ; LookOnTarget
  (:`Started`
    (if (`self.bIsLookOnTarget`)
      (set `self.bIsLookOnTarget` false)
      (else
        (`self.LockOnEnemy`)))))

(event `EnhancedInput|/Game/Input/IA_Look`
  (params (ActionValue :type "Vector2D Structure") (ElapsedSeconds :type "Float (double-precision)") (TriggeredSeconds :type "Float (double-precision)") (InputAction :type "InputAction Object Reference" :default "/Game/Input/IA_Look.IA_Look"))
  (bind _springarm (`self.SpringArm`))
  (bind (_returnvalue_roll _returnvalue_pitch _returnvalue_yaw) (`KismetMathLibrary.BreakRotator` (`SceneComponent.K2_GetComponentRotation` _springarm)))
  (bind (_relativerotation_roll _relativerotation_pitch _relativerotation_yaw) (`KismetMathLibrary.BreakRotator` (`SceneComponent.RelativeRotation` _springarm)))
  ; BaseMove
  (:`Triggered`
    (if (not (`self.bIsLookOnTarget`))
      (`SceneComponent.K2_SetWorldRotation` _springarm (`KismetMathLibrary.MakeRotator` 0.0 _returnvalue_pitch (+ _returnvalue_yaw ActionValue_X)) false false)
      (`SceneComponent.K2_SetRelativeRotation` _springarm (`KismetMathLibrary.MakeRotator` 0.0 (`KismetMathLibrary.FClamp` (+ (* ActionValue_Y -1.0) _relativerotation_pitch) -80.0 50.0) _relativerotation_yaw) false false)
      (else
        (set `self.OnTargetChangeEnemCurrentCursorDistance` (+ ActionValue_X (`self.OnTargetChangeEnemCurrentCursorDistance`)))))))

(event `EnhancedInput|/Game/Input/IA_Move`
  (params (ActionValue :type "Vector2D Structure") (ElapsedSeconds :type "Float (double-precision)") (TriggeredSeconds :type "Float (double-precision)") (InputAction :type "InputAction Object Reference" :default "/Game/Input/IA_Move.IA_Move"))
  (bind _returnvalue (!= ActionValue_X 0.0))
  (bind (_returnvalue_roll _returnvalue_pitch _returnvalue_yaw) (`KismetMathLibrary.BreakRotator` (`SceneComponent.K2_GetComponentRotation` (`self.Camera`))))
  (bind (_returnvalue_roll_2 _returnvalue_pitch_2 _returnvalue_yaw_2) (`KismetMathLibrary.BreakRotator` (`SceneComponent.K2_GetComponentRotation` (`self.Camera`))))
  ; BaseMove
  (:`Triggered`
    (`self.AddMovementInput` (`KismetMathLibrary.GetRightVector` (`KismetMathLibrary.MakeRotator` _returnvalue_roll_2 0.0 _returnvalue_yaw_2)) ActionValue_X)
    (`self.AddMovementInput` (`KismetMathLibrary.GetForwardVector` (`KismetMathLibrary.MakeRotator` 0.0 0.0 _returnvalue_yaw)) ActionValue_Y)
    (if (`self.bIsBackRight`)
      (`self.BackRightLeftCheck` ActionValue_X ActionValue_Y
        (:`Right`
          _)
        (:`Left`
          (set `self.PlayerMoveCameraRotation2BaseRotation_SpeedIn` 0.0 :!label _label_2)))
      (else
        (`self.BackRightLeftCheck` ActionValue_X ActionValue_Y
          (:`Right`
            (goto _label_2))
          (:`Left`
            _))))
    (`self.BackRightLeftCheck` ActionValue_X ActionValue_Y
      (:`Right`
        (set `self.bIsBackRight` true))
      (:`Left`
        (set `self.bIsBackRight` false)))
    (if (or _returnvalue (and _returnvalue (> ActionValue_Y 0.0)))
      (set `self.bIsCameraMove` true)
      (else
        (set `self.bIsCameraMove` false))))
  (:`Started`
    (set `self.PlayerMoveCameraRotation2BaseRotation_SpeedIn` 0.0))
  (:`Completed`
    (set `self.bIsCameraMove` false)))

(event `EnhancedInput|/Game/Input/IA_Jump`
  (params (ActionValue :type Boolean) (ElapsedSeconds :type "Float (double-precision)") (TriggeredSeconds :type "Float (double-precision)") (InputAction :type "InputAction Object Reference" :default "/Game/Input/IA_Jump.IA_Jump"))
  ; BaseMove
  (:`Started`
    (`self.Jump`)))

(event `EnhancedInput|/Game/Input/IA_Sprint`
  (params (ActionValue :type Boolean) (ElapsedSeconds :type "Float (double-precision)") (TriggeredSeconds :type "Float (double-precision)") (InputAction :type "InputAction Object Reference" :default "/Game/Input/IA_Sprint.IA_Sprint"))
  ; BaseMove
  (:`Started`
    (set `CharacterMovementComponent.MaxWalkSpeed` (`self.BaseSprintSpeed`) (`self.CharacterMovement`))
    (set `self.bIsSprint` true))
  (:`Completed`
    (set `CharacterMovementComponent.MaxWalkSpeed` (`self.BaseWalkSpeed`) (`self.CharacterMovement`))
    (set `self.bIsSprint` false)))

(fn `UserConstructionScript`)